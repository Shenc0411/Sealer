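; Player controller for the Sealer game that creates the HUD and handles rift sealing, level restart and return to the start menu.
; Holding SealRift while a rift is in range starts a timer and a looping sound; releasing cancels both, and completion calls Seal on the rift.
; Tick counts SealingTimeLeft down during sealing, and it resets from the character's SealingTime on start, cancel or finish.
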(event `self.ReceiveBeginPlay`
  (bind _assealer_player_character (cast `/Game/Blueprints/SealerPlayerCharacter` (`self.K2_GetPawn`)))
  (set `self.PlayerCharacterReference` _assealer_player_character)
  (bind _assealer_game_mode (cast `/Game/Blueprints/SealerGameMode` (`GameplayStatics.GetGameMode`)))
  (set `self.GameModeReference` _assealer_game_mode)
  (set `self.SealingTimeLeft` (`/Game/Blueprints/SealerPlayerCharacter.SealingTime` (`self.PlayerCharacterReference`)))
  (set `self.IsSealingRift` false)
  (bind _returnvalue (`|CreateWidget` "/Game/Blueprints/Widgets/GameHUD.GameHUD_C" self))
  (bind _output_get (set `self.GameHUDReference` _returnvalue))
  (`UserWidget.AddToViewport` _output_get 0))

(event `InputAction|RestartLevel`
  (params (Key :type "Key Structure"))
  (:`Pressed`
    (`/Game/Blueprints/SealerGameMode.RestartLevel` (`self.GameModeReference`))))

(event `InputAction|SealRift`
  (params (Key :type "Key Structure"))
  (bind _sealingtimerhandle (`self.SealingTimerHandle`))
  (bind _playercharacterreference (`self.PlayerCharacterReference`))
  (bind _returnvalue (`KismetSystemLibrary.K2_IsValidTimerHandle` _sealingtimerhandle))
  (:`Pressed`
    (if (not _returnvalue)
      (`/Engine/EditorBlueprintResources/StandardMacros.IsValid` (`/Game/Blueprints/SealerPlayerCharacter.RiftInRange` _playercharacterreference)
        (:`Is Valid`
          (bind _returnvalue_2 (`KismetSystemLibrary.K2_SetTimerDelegate` (delegate `FinishSealRift`) (`/Game/Blueprints/SealerPlayerCharacter.SealingTime` _playercharacterreference)))
          (set `self.SealingTimerHandle` _returnvalue_2)
          (set `self.SealingTimeLeft` (`/Game/Blueprints/SealerPlayerCharacter.SealingTime` (`self.PlayerCharacterReference`)))
          (set `self.IsSealingRift` true)
          (bind _returnvalue_3 (`GameplayStatics.SpawnSoundAtLocation` "/Game/Audio/LoopBeforeFinishSealing.LoopBeforeFinishSealing" (`self.K2_GetActorLocation`) (struct) 3.0 1.0 0.0 null null))
          (set `self.SealingSoundReference` _returnvalue_3)))))
  (:`Released`
    (if _returnvalue
      (`KismetSystemLibrary.K2_ClearAndInvalidateTimerHandle` _sealingtimerhandle)
      (set `self.SealingTimeLeft` (`/Game/Blueprints/SealerPlayerCharacter.SealingTime` (`self.PlayerCharacterReference`)))
      (set `self.IsSealingRift` false)
      (`ActorComponent.K2_DestroyComponent` (`self.SealingSoundReference`)))))

(event `FinishSealRift`
  (bind _playercharacterreference (`self.PlayerCharacterReference`))
  (`/Game/Blueprints/Rift.Seal` (`/Game/Blueprints/SealerPlayerCharacter.RiftInRange` _playercharacterreference) self _playercharacterreference)
  (`KismetSystemLibrary.K2_ClearAndInvalidateTimerHandle` (`self.SealingTimerHandle`))
  (set `self.SealingTimeLeft` (`/Game/Blueprints/SealerPlayerCharacter.SealingTime` (`self.PlayerCharacterReference`)))
  (set `self.IsSealingRift` false)
  (`ActorComponent.K2_DestroyComponent` (`self.SealingSoundReference`)))

(event `self.ReceiveTick`
  (params (DeltaSeconds :type "Float (single-precision)"))
  (bind _sealingtimeleft (`self.SealingTimeLeft`))
  (if (`self.IsSealingRift`)
    (set `self.SealingTimeLeft` (`KismetMathLibrary.FClamp` (- _sealingtimeleft DeltaSeconds) 0.0 _sealingtimeleft))))

(event `InputAction|ShowMainMenu`
  (params (Key :type "Key Structure"))
  (:`Pressed`
    (bind _assealer_game_instance (cast `/Game/Blueprints/SealerGameInstance` (`GameplayStatics.GetGameInstance`)))
    (`/Game/Blueprints/SealerGameInstance.BackToStartMenuLevel` _assealer_game_instance)))

(fn `UserConstructionScript`)