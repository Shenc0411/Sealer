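; Game mode for a rift-sealing game in which the level switches between two worlds.
; Switching toggles the current world, then shows and enables collision only on environment-tagged actors carrying that world's tag, hiding the rest; this also runs at BeginPlay.
; It also increments the game state's sealed-rift count, creates and removes each player controller's sealing prompt widget, and restarts the level by console command.
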(event `self.ReceiveBeginPlay`
  (`self.RefreshEnvironmentObjects`))

(event `RestartLevel`
  (`KismetSystemLibrary.ExecuteConsoleCommand` "RestartLevel" null))

(event `SwitchWorld`
  (set `self.CurrentWorld` (select `/Game/Blueprints/World_Enum` (`self.CurrentWorld`) :`NewEnumerator0` "NewEnumerator1" :`NewEnumerator1` "NewEnumerator0" :!type "/Game/Blueprints/World_Enum Enum"))
  (`self.RefreshEnvironmentObjects`))

(event `NotifyRiftSealed`
  (params (RiftReference :type "/Game/Blueprints/Rift Object Reference") (Instigator :type "/Game/Blueprints/SealerPlayerController Object Reference") (SealerCharacter :type "/Game/Blueprints/SealerPlayerCharacter Object Reference"))
  (bind _assealer_game_state (cast `/Game/Blueprints/SealerGameState` (`GameplayStatics.GetGameState`)))
  (set `/Game/Blueprints/SealerGameState.NumberOfRiftsSealed` (+ (`/Game/Blueprints/SealerGameState.NumberOfRiftsSealed` _assealer_game_state) 1) _assealer_game_state))

(event `ShowSealingPrompt`
  (params (PlayerController :type "/Game/Blueprints/SealerPlayerController Object Reference"))
  (bind _sealingpromptreference (`/Game/Blueprints/SealerPlayerController.SealingPromptReference` PlayerController))
  (`/Engine/EditorBlueprintResources/StandardMacros.IsValid` _sealingpromptreference
    (:`Is Valid`
      (`Widget.RemoveFromParent` _sealingpromptreference))
    (:`Is Not Valid`
      _))
  (bind _returnvalue (`|CreateWidget` "/Game/Blueprints/Widgets/SealingPrompt.SealingPrompt_C" PlayerController))
  (bind _output_get (set `/Game/Blueprints/SealerPlayerController.SealingPromptReference` _returnvalue PlayerController))
  (`UserWidget.AddToViewport` _output_get 0))

(event `HideSealingPrompt`
  (params (PlayerController :type "/Game/Blueprints/SealerPlayerController Object Reference"))
  (bind _sealingpromptreference (`/Game/Blueprints/SealerPlayerController.SealingPromptReference` PlayerController))
  (`/Engine/EditorBlueprintResources/StandardMacros.IsValid` _sealingpromptreference
    (:`Is Valid`
      (`Widget.RemoveFromParent` _sealingpromptreference))))

(fn `RefreshEnvironmentObjects`
  (bind _outactors (`GameplayStatics.GetAllActorsWithTag` (`self.EnvironmentObjectTag`)))
  (for _array_element _outactors
    (bind _returnvalue (`self.ActorHasTag` _array_element (`self.WorldEnumToTag` (`self.CurrentWorld`))))
    (`self.SetActorHiddenInGame` _array_element (not _returnvalue))
    (`self.SetActorEnableCollision` _array_element _returnvalue)))

(fn `UserConstructionScript`)

(fn `WorldEnumToTag`
  (params (WorldEnum :type "/Game/Blueprints/World_Enum Enum" :default "NewEnumerator0"))
  (returns (Tag :type Name))
  (return (select `/Game/Blueprints/World_Enum` WorldEnum :`NewEnumerator0` "World0" :`NewEnumerator1` "World1" :!type "Name")))