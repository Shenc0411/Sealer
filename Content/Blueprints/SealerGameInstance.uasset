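; SealerGameInstance is a Game Instance Blueprint that manages level progression and opens the main menu.
; It keeps an array of level structs holding a name and unlock flag, plus the current level index.
; GoToNextLevel advances the index, unlocks that entry and calls ChangeToLevel, which only opens unlocked levels.
; Locked requests and the end of the list only print a message.
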(event `ChangeToLevel`
  (params (LevelIndex :type Integer))
  (bind (_isunlocked _levelname) (break `/Game/Blueprints/LevelStruct` (`|GetArrayItem` (`self.Levels`) LevelIndex)))
  (if _isunlocked
    (`GameplayStatics.OpenLevel` _levelname)
    (else
      (`KismetSystemLibrary.PrintString` "Cannot Switch to a locked level"))))

(event `ShowMainMenu`
  (bind _returnvalue (`GameplayStatics.GetPlayerController` 0))
  (bind _returnvalue_2 (`|CreateWidget` "/Game/Blueprints/Widgets/MainMenu.MainMenu_C" _returnvalue))
  (`UserWidget.AddToViewport` _returnvalue_2 0)
  (set `PlayerController.bShowMouseCursor` true _returnvalue))

(event `GoToNextLevel`
  (bind _levels (`self.Levels`))
  (bind _returnvalue (+ (`self.CurrentLevel`) 1))
  (if (< _returnvalue (`KismetArrayLibrary.Array_Length` _levels))
    (bind _output_get (set `self.CurrentLevel` _returnvalue))
    (`KismetArrayLibrary.Array_Set` _levels _output_get (make `/Game/Blueprints/LevelStruct` true (`.LevelName_4_121B13A94870EAB500E32CBCE30325DF` (break `/Game/Blueprints/LevelStruct` (`|GetArrayItem` _levels _output_get)))))
    (`self.ChangeToLevel` _output_get)
    (else
      (`KismetSystemLibrary.PrintString` "End of Game" true true (struct :`R` 1.0 :`B` 0.052632 :`A` 1.0)))))