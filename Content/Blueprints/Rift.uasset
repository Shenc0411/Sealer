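; Rift actor that flips the player between worlds on contact and can be sealed.
; Touching the inner box calls SwitchWorld on the GameMode and teleports the player along X to the rift's far side.
; A separate sealing box registers the rift on the player, toggles the sealing prompt and fades the rift sound.
; Seal notifies the GameMode, plays a finishing sound and destroys the rift.
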(event `self.Box.OnComponentBeginOverlap`
  (params (OverlappedComponent :type "PrimitiveComponent Object Reference") (OtherActor :type "Actor Object Reference") (OtherComp :type "PrimitiveComponent Object Reference") (OtherBodyIndex :type Integer) (bFromSweep :type Boolean) (SweepResult :type "HitResult Structure (by ref)"))
  (bind _assealer_player_character (cast `/Game/Blueprints/SealerPlayerCharacter` OtherActor))
  (bind _assealer_game_mode (cast `/Game/Blueprints/SealerGameMode` (`GameplayStatics.GetGameMode`)))
  (`/Game/Blueprints/SealerGameMode.SwitchWorld` _assealer_game_mode)
  (bind _returnvalue (`self.K2_GetActorLocation` _assealer_player_character))
  (if (< (.x _returnvalue) (.x (`self.K2_GetActorLocation` self)))
    (`self.K2_SetActorLocation` _assealer_player_character (+ _returnvalue (`KismetMathLibrary.MakeVector` (`self.TeleportXOffset`))) false true)
    (else
      (`self.K2_SetActorLocation` _assealer_player_character (+ _returnvalue (`KismetMathLibrary.MakeVector` (- 0.0 (`self.TeleportXOffset`)))) false true))))

(event `Seal`
  (params (Instigator :type "/Game/Blueprints/SealerPlayerController Object Reference") (SealerCharacter :type "/Game/Blueprints/SealerPlayerCharacter Object Reference"))
  (bind _assealer_game_mode (cast `/Game/Blueprints/SealerGameMode` (`GameplayStatics.GetGameMode`)))
  (`/Game/Blueprints/SealerGameMode.NotifyRiftSealed` _assealer_game_mode self null null)
  (`GameplayStatics.PlaySoundAtLocation` "/Game/Audio/SealingFinished.SealingFinished" (`self.K2_GetActorLocation`) (struct) 1.0 1.0 0.0 null null null)
  (`self.K2_DestroyActor`))

(event `self.SealingCollisionBox.OnComponentBeginOverlap`
  (params (OverlappedComponent :type "PrimitiveComponent Object Reference") (OtherActor :type "Actor Object Reference") (OtherComp :type "PrimitiveComponent Object Reference") (OtherBodyIndex :type Integer) (bFromSweep :type Boolean) (SweepResult :type "HitResult Structure (by ref)"))
  (bind _assealer_player_character (cast `/Game/Blueprints/SealerPlayerCharacter` OtherActor))
  (set `/Game/Blueprints/SealerPlayerCharacter.RiftInRange` self _assealer_player_character)
  (bind _assealer_game_mode (cast `/Game/Blueprints/SealerGameMode` (`GameplayStatics.GetGameMode`)))
  (bind _assealer_player_controller (cast `/Game/Blueprints/SealerPlayerController` (`Pawn.GetController` _assealer_player_character)))
  (`/Game/Blueprints/SealerGameMode.ShowSealingPrompt` _assealer_game_mode _assealer_player_controller self)
  (bind _returnvalue (`GameplayStatics.SpawnSoundAtLocation` "/Game/Audio/RiftSFX.RiftSFX" (`self.K2_GetActorLocation`) (struct) 1.0 1.0 0.0 null null))
  (bind _output_get (set `self.RiftSFXReference` _returnvalue))
  (`AudioComponent.FadeIn` _output_get 1.0 1.0 0.0))

(event `self.SealingCollisionBox.OnComponentEndOverlap`
  (params (OverlappedComponent :type "PrimitiveComponent Object Reference") (OtherActor :type "Actor Object Reference") (OtherComp :type "PrimitiveComponent Object Reference") (OtherBodyIndex :type Integer))
  (bind _assealer_player_character (cast `/Game/Blueprints/SealerPlayerCharacter` OtherActor))
  (set `/Game/Blueprints/SealerPlayerCharacter.RiftInRange` null _assealer_player_character)
  (bind _assealer_game_mode (cast `/Game/Blueprints/SealerGameMode` (`GameplayStatics.GetGameMode`)))
  (bind _assealer_player_controller (cast `/Game/Blueprints/SealerPlayerController` (`Pawn.GetController` _assealer_player_character)))
  (`/Game/Blueprints/SealerGameMode.HideSealingPrompt` _assealer_game_mode _assealer_player_controller self)
  (`AudioComponent.FadeOut` (`self.RiftSFXReference`) 0.5 0.0))

(fn `UserConstructionScript`)